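; BP_FlashingCube is a Blueprint cube that flashes random glowing colours, like a disco light.
; Its DISCO function runs from the Construction Script and on every Tick.
; Each call creates a new dynamic instance of MI_BetterWood on the Cube, rather than reusing one.
; It then sets a high glow intensity, a black secondary colour and random Red, Green and Blue parameters.
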(event EventTick
  (params (DeltaSeconds :type Float%20%28single-precision%29))
  (CallFunction|DISCO))

(event EventBeginPlay)

(fn ConstructionScript
  (CallFunction|DISCO))

(fn DISCO
  (bind _returnvalue (Rendering|Material|CreateDynamicMaterialInstance (Variables|Default|GetCube) 0 "/Game/Materials/MI_BetterWood.MI_BetterWood" "None" :!class /Script/Engine.PrimitiveComponent))
  (Rendering|Material|SetScalarParameterValue _returnvalue "GlowingIntensity" 5e+03 :!class /Script/Engine.MaterialInstanceDynamic)
  (Rendering|Material|SetVectorParameterValue _returnvalue "OtherColour" "(R=0.000000,G=0.000000,B=0.000000,A=1.000000)" :!class /Script/Engine.MaterialInstanceDynamic)
  (Rendering|Material|SetScalarParameterValue _returnvalue "Red" (Math|Random|RandomFloatinRange 0.0 1.0) :!class /Script/Engine.MaterialInstanceDynamic)
  (Rendering|Material|SetScalarParameterValue _returnvalue "Green" (Math|Random|RandomFloatinRange 0.0 1.0) :!class /Script/Engine.MaterialInstanceDynamic)
  (Rendering|Material|SetScalarParameterValue _returnvalue "Blue" (Math|Random|RandomFloatinRange 0.0 1.0) :!class /Script/Engine.MaterialInstanceDynamic))