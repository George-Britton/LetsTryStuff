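; Crocalor actor that appears to be a sandbox for timers, event dispatchers and audio.
; Handlers count bell rings with a timed reset, print damage and greetings, and pause/resume audio.
; A war-crime event broadcasts, plays audio and swaps the sprite, while a random Spiderman check can cancel its timer.
; All setup that binds these handlers, starts timers or creates the widget is disconnected, so never runs.
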(event Custom|CustomEvent_0
  (bind _audio (Variables|Default|GetAudio))
  (Audio|Components|Audio|Play _audio 15.0)
  (Class|AudioComponent|SetPaused _audio true)
  (Utilities|Time|SetTimerbyEvent (delegate Custom|CustomEvent_2) 3.0))

(event Custom|CustomEvent_1
  (Development|PrintString "Crocalor says hi"))

(event Custom|OnTakeAnyDamage_Event_0
  (params (DamagedActor :type Actor%20Object%20Reference) (Damage :type Float%20%28single-precision%29) (DamageType :type Damage%20Type%20Object%20Reference) (InstigatedBy :type Controller%20Object%20Reference) (DamageCauser :type Actor%20Object%20Reference))
  (Development|PrintString (Utilities|String|Append "Haha you took " (Utilities|String|ToString(Float) Damage) " damage")))

(event Custom|OnDestroyed_Event_0
  (params (DestroyedActor :type Actor%20Object%20Reference))
  (bind _asbp_ed (Utilities|Casting|CastToBP_ED DestroyedActor))
  (EventDispatchers|UnbindEventfromOnEvent _asbp_ed (delegate Custom|CustomEvent_1)))

(event Custom|CustomEvent_2
  (Class|AudioComponent|SetPaused (Variables|Default|GetAudio) false))

(event Custom|Commit%20War%20Crime
  (Default|CallOnWarCrime 3)
  (Utilities|Time|ClearandInvalidateTimerbyHandle (Variables|Default|GetSpideyTimer))
  (Audio|Components|Audio|Play (Variables|Default|GetAudio) 2.0)
  (Rendering|Components|Sprite|SetSprite (Variables|Default|GetPaperSprite) "/Game/2D/CrocStache_Sprite.CrocStache_Sprite"))

(event Custom|Spidey%20Saves%20the%20Day
  (if (> (Math|Random|RandomIntegerinRange 0 99) 10)
    (Utilities|Time|ClearandInvalidateTimerbyHandle (Variables|Default|GetSpideyTimer))
    (Utilities|Time|ClearandInvalidateTimerbyHandle (Variables|Default|GetWarCrimeTimer))
    (Development|PrintString "Woo Spiderman" true true "(R=0.000000,G=0.660000,B=1.000000,A=1.000000)" 9999.0)))

(event Custom|ResetBells
  (Development|PrintString "Bells are reset")
  (Variables|Default|SetBellsRung 0))

(event Custom|RingBell
  (Math|Integer|IncrementInt (Variables|Default|GetBellsRung)
    (:%20%20
      (if (Utilities|Time|IsValidTimerHandle (Variables|Default|GetBellResetTimer))
        (if (== (Variables|Default|GetBellsRung) 3)
          (Utilities|Time|ClearandInvalidateTimerbyHandle (Variables|Default|GetBellResetTimer)))
        (else
          (bind _returnvalue (Utilities|Time|SetTimerbyEvent (delegate Custom|ResetBells) 5.0))
          (Variables|Default|SetBellResetTimer _returnvalue))))))

(fn ConstructionScript)

(fn BreakProtocol3
  (Development|PrintString "hehehe"))